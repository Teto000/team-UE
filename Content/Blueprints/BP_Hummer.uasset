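; BP_Hummer is a player-controlled hammer actor for striking BP_Mole targets, whack-a-mole style.
; Tick moves the skeletal mesh by scaled mouse axis input and keeps a sphere at a fixed offset from it.
; Left click sets a Hit flag that makes Tick play HitTimeline, animating mesh pitch until it finishes and resets.
; Any capsule overlap with a mole calls its OnCollision, without checking the Hit flag.
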(event `self.ReceiveBeginPlay`
  (`self.EnableInput` (`GameplayStatics.GetPlayerController` 0))
  (set `self.bHit` false))

(event `self.ReceiveTick`
  (params (DeltaSeconds :type "Float (single-precision)"))
  (bind (_defaltrot_roll _defaltrot_pitch _defaltrot_yaw) (`KismetMathLibrary.BreakRotator` (`self.DefaltRot`)))
  (bind (_relativelocation_x _relativelocation_y _relativelocation_z) (`KismetMathLibrary.BreakVector` (`SceneComponent.RelativeLocation` (`self.SkeletalMesh`))))
  (bind (_relativelocation_x_2 _relativelocation_y_2 _relativelocation_z_2) (`KismetMathLibrary.BreakVector` (`SceneComponent.RelativeLocation` (`self.SkeletalMesh`))))
  ;[1 1 1] マウスを使った移動処理
  (`SceneComponent.K2_SetRelativeLocation` (`self.SkeletalMesh`) (`KismetMathLibrary.MakeVector` (+ _relativelocation_x_2 (* (`self.GetInputAxisValue`) 10.0)) (+ _relativelocation_y_2 (* (`self.GetInputAxisValue`) 10.0)) _relativelocation_z_2) false false)
  (`SceneComponent.K2_SetRelativeLocation` (`self.Sphere`) (`KismetMathLibrary.MakeVector` (+ _relativelocation_x 130.0) _relativelocation_y (+ _relativelocation_z -80.0)) false false)
  (if (`self.bHit`)
    (bind (_direction _newtrack_0) (`Timeline|HitTimeline` :!label _label)
      (:`Update`
        (`SceneComponent.K2_SetRelativeRotation` (`self.SkeletalMesh`) (`KismetMathLibrary.MakeRotator` _defaltrot_roll _newtrack_0 _defaltrot_yaw) false false))
      (:`Finished`
        (set `self.bHit` false)
        (goto _label :!via `SetNewTime`)))))

(event `Key|LeftMouseButton`
  (params (Key :type "Key Structure"))
  ;[1 1 1] 叩く処理
  (:`Pressed`
    (set `self.bHit` true)))

(event `self.Capsule.OnComponentBeginOverlap`
  (params (OverlappedComponent :type "PrimitiveComponent Object Reference") (OtherActor :type "Actor Object Reference") (OtherComp :type "PrimitiveComponent Object Reference") (OtherBodyIndex :type Integer) (bFromSweep :type Boolean) (SweepResult :type "HitResult Structure (by ref)"))
  (bind _asbp_mole (cast `/Game/Blueprints/BP_Mole` (`ActorComponent.GetOwner` OtherComp)))
  (`/Game/Blueprints/BP_Mole.OnCollision` _asbp_mole))

(fn `UserConstructionScript`)