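; BP_Mole is a whack-a-mole target that rises along a timeline after a random tick countdown, then rerolls its type.
; A weighted roll picks normal, double, bomb or special, setting material and score, with bombs costing points.
; OnCollision plays hit effects and returns points once per cycle.
; Double moles need two hits, with a brief tick-counted invulnerability after the first.
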(event `self.ReceiveBeginPlay`
  (bind (_returnvalue_x _returnvalue_y _returnvalue_z) (`KismetMathLibrary.BreakVector` (`self.K2_GetActorLocation`)))
  (set `self.nDelay` (`KismetMathLibrary.RandomIntegerInRange` 60 800))
  (set `self.fStartingHeight` _returnvalue_z)
  (set `self.bReady` true)
  (set `self.bStartMove` false)
  (`self.SetNewType`)
  (`self.Set Material`)
  (set `self.nLife` 0)
  (set `self.bDamaged` false))

(event `self.ReceiveTick`
  (params (DeltaSeconds :type "Float (single-precision)"))
  (bind (_returnvalue_x _returnvalue_y) (`KismetMathLibrary.BreakVector` (`self.K2_GetActorLocation`)))
  (bind _ninvulnerability (`self.nInvulnerability`))
  (if (not (<= _ninvulnerability 0))
    (bind _result (`/Engine/EditorBlueprintResources/StandardMacros.DecrementInt` _ninvulnerability)
      (:`  `
        (set `self.nInvulnerability` _result))))
  (if (`self.bStartMove`)
    (bind (_direction _newtrack_0) (`Timeline|Timeline_0` :!label _label)
      (:`Update`
        (`self.K2_SetActorLocation` (`KismetMathLibrary.MakeVector` _returnvalue_x _returnvalue_y (+ _newtrack_0 (`self.fStartingHeight`)))))
      (:`Finished`
        (set `self.bReady` true)
        (set `self.bStartMove` false)
        (set `self.nLife` 0)
        (set `self.bDamaged` false)
        (`self.SetNewType`)
        (`self.Set Material`)
        (set `self.nDelay` (`KismetMathLibrary.RandomIntegerInRange` 120 360))
        (goto _label :!via `SetNewTime`)))
    (elif (`self.bReady`)
      (bind _result_2 (`/Engine/EditorBlueprintResources/StandardMacros.DecrementInt` (`self.nDelay`))
        (:`  `
          (if (<= _result_2 0)
            (set `self.bStartMove` true)
            (else
              (set `self.nDelay` _result_2))))))))

(fn `GetPoints`
  (returns (NewParam :type Integer))
  (if (== (`self.nType`) 0)
    (return 1)
    (elif (== (`self.nType`) 1)
      (return 3)
      (elif (== (`self.nType`) 2)
        (return -3)
        (else
          (return 5))))))

(fn `NewFunction_0`
  (returns (NewParam :type Integer))
  (return (`self.nType`)))

(fn `OnCollision`
  (returns (NewParam :type Integer))
  (bind (_returnvalue_x _returnvalue_y _returnvalue_z) (`KismetMathLibrary.BreakVector` (`self.K2_GetActorLocation`)))
  (bind _staticmesh (`self.StaticMesh`))
  (bind _staticmesh_2 (`self.StaticMesh`))
  (bind _staticmesh_3 (`self.StaticMesh`))
  (`GameplayStatics.PlaySound2D` "/Game/SE/中パンチ__online-audio-converter_com_.中パンチ__online-audio-converter_com_" 1.0 1.0 0.0 null null)
  (`GameplayStatics.SpawnEmitterAtLocation` "/Game/particle/star.star" (`KismetMathLibrary.MakeVector` _returnvalue_x _returnvalue_y (+ _returnvalue_z 100.0)))
  (if (<= (`self.nInvulnerability`) 0)
    (if (`self.bDamaged`)
      (return 0)
      (elif (== (`self.nType`) 1)
        (if (>= (`self.nLife`) 1)
          (`KismetArrayLibrary.Array_Remove` (`MeshComponent.GetMaterials` _staticmesh_3))
          (`PrimitiveComponent.SetMaterial` _staticmesh_3 0 "/Game/Materials/MoleMaterials/DamagedMaterial.DamagedMaterial")
          (set `self.bDamaged` true)
          (bind _newparam (`self.GetPoints`))
          (return _newparam)
          (else
            (`/Engine/EditorBlueprintResources/StandardMacros.IncrementInt` (`self.nLife`)
              (:`  `
                (`KismetArrayLibrary.Array_Remove` (`MeshComponent.GetMaterials` _staticmesh_2))
                (`PrimitiveComponent.SetMaterial` _staticmesh_2 0 "/Game/Materials/MoleMaterials/DoubleMoleMaterialBroken.DoubleMoleMaterialBroken")
                (set `self.nInvulnerability` 20)
                (return 0)))))
        (else
          (`KismetArrayLibrary.Array_Remove` (`MeshComponent.GetMaterials` _staticmesh))
          (`PrimitiveComponent.SetMaterial` _staticmesh 0 "/Game/Materials/MoleMaterials/DamagedMaterial.DamagedMaterial")
          (set `self.bDamaged` true)
          (bind _newparam_2 (`self.GetPoints`))
          (return _newparam_2))))))

(fn `Set Material`
  (bind _staticmesh (`self.StaticMesh`))
  (bind _staticmesh_2 (`self.StaticMesh`))
  (bind _staticmesh_3 (`self.StaticMesh`))
  (bind _staticmesh_4 (`self.StaticMesh`))
  (if (== (`self.nType`) 0)
    (`KismetArrayLibrary.Array_Remove` (`MeshComponent.GetMaterials` _staticmesh_2))
    (`PrimitiveComponent.SetMaterial` _staticmesh_2 0 "/Game/Materials/MoleMaterials/NormalMoleMaterial.NormalMoleMaterial")
    (elif (== (`self.nType`) 1)
      (`KismetArrayLibrary.Array_Remove` (`MeshComponent.GetMaterials` _staticmesh_3))
      (`PrimitiveComponent.SetMaterial` _staticmesh_3 0 "/Game/Materials/MoleMaterials/DoubleMoleMaterial.DoubleMoleMaterial")
      (elif (== (`self.nType`) 2)
        (`KismetArrayLibrary.Array_Remove` (`MeshComponent.GetMaterials` _staticmesh_4))
        (`PrimitiveComponent.SetMaterial` _staticmesh_4 0 "/Game/Materials/MoleMaterials/BombMoleMaterial.BombMoleMaterial")
        (else
          (`KismetArrayLibrary.Array_Remove` (`MeshComponent.GetMaterials` _staticmesh))
          (`PrimitiveComponent.SetMaterial` _staticmesh 0 "/Game/Materials/MoleMaterials/SpecialMoleMaterial.SpecialMoleMaterial"))))))

(fn `SetNewType`
  (bind _output_get (set `self.nNumber` (`KismetMathLibrary.RandomIntegerInRange` 0 100)))
  (if (<= _output_get 65)
    (set `self.nType` 0)
    (elif (<= _output_get 75)
      (set `self.nType` 1)
      (elif (<= _output_get 95)
        (set `self.nType` 2)
        (else
          (set `self.nType` 3))))))

(fn `UserConstructionScript`)